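; BP_DialogueComponent lets a player hold a dialogue with its owning NPC, driven by a behavior tree.
; On BeginPlay it spawns a dedicated dialogue AI controller, fed from NPC and player data assets plus the owner's audio component.
; Interaction opens the dialogue widget, switches input to UI, runs the tree and passes the widget through the blackboard.
; The widget's exit callback stops the tree, removes the widget and restores player control.
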(event Custom|OnExit_Event
  (bind _dialoguewidget (Variables|Default|GetDialogueWidget))
  (bind _returnvalue (Widget|GetOwningPlayer _dialoguewidget))
  (Input|SetInputModeGameOnly _returnvalue false)
  (Variables|/Script/Engine.PlayerController|SetbShowMouseCursor _returnvalue false)
  (AI|Logic|StopLogic (Variables|/Script/AIModule.AIController|GetBrainComponent (Variables|Default|GetAIController)) "Dialogue Exited")
  (Widget|RemovefromParent _dialoguewidget)
  (Input|EnableInput (stale EventOnInteraction PlayerCharacter) (.AsPlayer%20Controller (Utilities|Casting|CastToPlayerController (Pawn|GetController (stale EventOnInteraction PlayerCharacter))))))

(event EventBeginPlay
  (bind _npcdataasset (Variables|Default|GetNPCDataAsset))
  (bind _returnvalue (Game|SpawnActorfromClass "/Game/DialogueSystem/BP_DialogueAIController.BP_DialogueAIController_C" (Math|Transform|MakeTransform "0, 0, 0" "0, 0, 0" "1.000000,1.000000,1.000000") "Undefined" "MultiplyWithRoot" 0 0))
  (bind _output_get (Variables|Default|SetAIController _returnvalue))
  (Variables|/Game/DialogueSystem/BP_DialogueAIController.BP_DialogueAIController_C|SetLevel _output_get (Variables|/Game/DialogueSystem/NPCDataAssets/CharacterDataAsset.CharacterDataAsset_C|GetLevel _npcdataasset))
  (Variables|/Game/DialogueSystem/BP_DialogueAIController.BP_DialogueAIController_C|SetName _output_get (Variables|/Game/DialogueSystem/NPCDataAssets/CharacterDataAsset.CharacterDataAsset_C|GetName _npcdataasset))
  (Variables|/Game/DialogueSystem/BP_DialogueAIController.BP_DialogueAIController_C|SetPlayerName _output_get (Variables|/Game/DialogueSystem/NPCDataAssets/CharacterDataAsset.CharacterDataAsset_C|GetName (Variables|Default|GetPlayerDataAsset)))
  (Variables|/Game/DialogueSystem/BP_DialogueAIController.BP_DialogueAIController_C|SetAudioSource _output_get (Actor|GetComponentbyClass (Components|GetOwner) "/Script/Engine.AudioComponent")))

(event EventOnInteraction
  (params (PlayerCharacter :type BP%20Third%20Person%20Character%20Object%20Reference))
  (bind _returnvalue (Pawn|GetController PlayerCharacter))
  (bind _aicontroller (Variables|Default|GetAIController))
  (bind _asplayer_controller (Utilities|Casting|CastToPlayerController _returnvalue))
  (bind _returnvalue_2 (UserInterface|CreateWidget "/Game/DialogueSystem/UI/BP_DialogueWidget.BP_DialogueWidget_C" _asplayer_controller))
  (bind _output_get (Variables|Default|SetDialogueWidget _returnvalue_2))
  (EventDispatchers|AssignOnExit _output_get (delegate Custom|OnExit_Event))
  (UserInterface|Viewport|AddtoViewport _output_get 0)
  (Input|SetInputModeGameandUI _asplayer_controller _output_get "DoNotLock" false false)
  (Input|DisableInput PlayerCharacter _asplayer_controller)
  (Variables|/Script/Engine.PlayerController|SetbShowMouseCursor _asplayer_controller true)
  (AI|RunBehaviorTree _aicontroller (Variables|Default|GetDialogueTree))
  (bind _blackboardcomponent (Class|AIController|UseBlackboard _aicontroller "/Game/DialogueSystem/DialogueTrees/BB_DialogueBlackboard.BB_DialogueBlackboard"))
  (AI|Components|Blackboard|SetValueasObject _blackboardcomponent (Utilities|Name|MakeLiteralName "DialogueWidget") (Variables|Default|GetDialogueWidget)))