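; BP_NPC is an NPC Blueprint that makes the character look at the player when the player comes within its detection cone.
; On BeginPlay it caches the mesh's ABP_Manny_Look anim instance.
; Overlaps between LookAtCone and BP_ThirdPersonCharacter toggle that anim Blueprint's LookAtPlayer flag, leaving the look behavior to the animation side.
; The construction script assigns LookAtCone a custom collision object channel.
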(event OnComponentBeginOverlap(LookAtCone)
  (params (OverlappedComponent :type Primitive%20Component%20Object%20Reference) (OtherActor :type Actor%20Object%20Reference) (OtherComp :type Primitive%20Component%20Object%20Reference) (OtherBodyIndex :type Integer) (bFromSweep :type Boolean) (SweepResult :type Hit%20Result%20Structure%20%28by%20ref%29))
  (Utilities|Casting|CastToBP_ThirdPersonCharacter OtherActor)
  (Variables|/Game/Characters/Mannequins/Animations/ABP_Manny_Look.ABP_Manny_Look_C|SetLookAtPlayer (Variables|Default|GetAnimBlueprint) true))

(event OnComponentEndOverlap(LookAtCone)
  (params (OverlappedComponent :type Primitive%20Component%20Object%20Reference) (OtherActor :type Actor%20Object%20Reference) (OtherComp :type Primitive%20Component%20Object%20Reference) (OtherBodyIndex :type Integer))
  (Utilities|Casting|CastToBP_ThirdPersonCharacter OtherActor)
  (Variables|/Game/Characters/Mannequins/Animations/ABP_Manny_Look.ABP_Manny_Look_C|SetLookAtPlayer (Variables|Default|GetAnimBlueprint) false))

(event EventBeginPlay
  (bind _asabp_manny_look (Utilities|Casting|CastToABP_Manny_Look (Components|SkeletalMesh|GetAnimInstance (Variables|Character|GetMesh))))
  (Variables|Default|SetAnimBlueprint _asabp_manny_look))

(fn ConstructionScript
  (Collision|SetCollisionObjectType (Variables|Default|GetLookAtCone) "ECC_GameTraceChannel1"))